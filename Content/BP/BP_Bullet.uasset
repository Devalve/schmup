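; BP_Bullet is a bullet actor that damages a referenced Enemy on a positional match.
; On BeginPlay it checks once whether its location equals the Enemy's within a tiny tolerance, with no collision or overlap events.
; A match subtracts the Enemy's own DamageToEnemy from its EnemyHealth and destroys the bullet.
; Otherwise it prints a Russian "something is wrong" debug message and stays in the world.
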(event `self.ReceiveBeginPlay`
  (bind _enemy (`self.Enemy`))
  (if (== (`self.K2_GetActorLocation`) (`self.K2_GetActorLocation` (`self.Enemy`)))
    (set `/Game/BP/BP_Enemy.EnemyHealth` (- (`/Game/BP/BP_Enemy.EnemyHealth` _enemy) (`/Game/BP/BP_Enemy.Damage To Enemy` _enemy)) _enemy)
    (`self.K2_DestroyActor`)
    (else
      (`KismetSystemLibrary.PrintString` "Что-то не так"))))

(fn `UserConstructionScript`)