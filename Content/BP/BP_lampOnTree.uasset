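; BP_lampOnTree is a lamp-on-tree actor, going by its name, that animates the rotation of a SpringArm from BeginPlay.
; A timeline runs at a rate of 1/Period from a StatsFrom start position, so speed and phase come from variables.
; Each update sets the arm's relative rotation to Amplitude times the degree cosine of the timeline track, using the spring arm as a pivot.
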(event `self.ReceiveBeginPlay`
  (bind _rotate_brocken_lattice (`self.rotate_brocken_lattice`))
  (`TimelineComponent.SetPlayRate` _rotate_brocken_lattice (/ 1.0 (`self.period`)))
  (`TimelineComponent.SetPlaybackPosition` _rotate_brocken_lattice (`self.stats from`) false true)
  (bind (_direction _newtrack_0) (`Timeline|rotate_brocken_lattice`)
    (:`Update`
      (`SceneComponent.K2_SetRelativeRotation` (`self.SpringArm`) (* (`self.amplitude`) (`KismetMathLibrary.DegCos` _newtrack_0)) false false))))

(fn `UserConstructionScript`)