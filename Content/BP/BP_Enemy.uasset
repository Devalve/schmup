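; BP_Enemy is an enemy actor that takes damage, hurts the player on contact and is destroyed when its health runs out.
; EnemyDamage subtracts incoming damage from EnemyHealth, printing the remaining health or a death message.
; Hits on the 2DSideScrollerCharacter apply damage through a DoOnce, reset after a short retriggerable delay as an attack cooldown.
; Tick spawns an actor at the Arrow's transform every frame, with no class shown.
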(event `self.ReceiveAnyDamage`
  (params (Damage :type "Float (single-precision)") (DamageType :type "DamageType Object Reference") (InstigatedBy :type "Controller Object Reference") (DamageCauser :type "Actor Object Reference"))
  ;[1 1 1] Comment
  (`self.Enemy Damage` Damage))

(event `self.ReceiveHit`
  (params (MyComp :type "PrimitiveComponent Object Reference") (Other :type "Actor Object Reference") (OtherComp :type "PrimitiveComponent Object Reference") (bSelfMoved :type Boolean) (HitLocation :type "Vector Structure") (HitNormal :type "Vector Structure") (NormalImpulse :type "Vector Structure") (Hit :type "HitResult Structure (by ref)"))
  ;[1 1 1] Comment
  (`/Engine/EditorBlueprintResources/StandardMacros.DoOnce` false :!label _label
    (:`Completed`
      (if (== (`GameplayStatics.GetObjectClass` Other) "/Game/2DSideScrollerBP/Blueprints/2DSideScrollerCharacter.2DSideScrollerCharacter_C")
        (`GameplayStatics.ApplyDamage` Other (`self.Damage`))
        (`KismetSystemLibrary.RetriggerableDelay` 0.2)
        (`self.ResetAttack`)))))

(event `ResetAttack`
  ;[1 1 1] Comment
  (goto _label :!via `Reset`))

(event `self.ReceiveTick`
  (params (DeltaSeconds :type "Float (single-precision)"))
  ;[1 1 1] Comment
  (`|SpawnActorFromClass` "/Game/BP/BP_EnemyBullet.BP_EnemyBullet_C" (`SceneComponent.K2_GetComponentToWorld` (`self.Arrow`)) "Undefined" "OverrideRootScale" null null))

(fn `Enemy Damage`
  (params (B :type "Float (double-precision)"))
  (bind _returnvalue (- (`self.EnemyHealth`) B))
  (if (> _returnvalue 0.0)
    (bind _output_get (set `self.EnemyHealth` _returnvalue))
    (`KismetSystemLibrary.PrintString` (`KismetStringLibrary.Conv_DoubleToString` _output_get))
    (else
      (`KismetSystemLibrary.PrintString` "ENEMY IS DEAD")
      (`self.K2_DestroyActor`))))

(fn `UserConstructionScript`)